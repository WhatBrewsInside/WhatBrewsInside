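; BP_Climbing is a climbable actor that carries the first-person player along a spline.
; Box overlap toggles the key prompt, actor input and a delay loop that yaws the Arrow toward the player to orient the spline path.
; ClimbingEvent moves the player along ClimbingPath with a Timeline, while a second Timeline tilts the camera down.
; Player input is disabled during the tilt and returns with camera control after a delay.
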(event OnComponentEndOverlap(Box)
  (params (OverlappedComponent :type Primitive%20Component%20Object%20Reference) (OtherActor :type Actor%20Object%20Reference) (OtherComp :type Primitive%20Component%20Object%20Reference) (OtherBodyIndex :type Integer))
  ;[0.15 0.15 0.15 0.5] Displaying controls
  (bind _asbp_first_person_character (Utilities|Casting|CastToBP_FirstPersonCharacter OtherActor))
  (Default|HiddenWidget _asbp_first_person_character "/Game/Climbing/ClimbingKey.ClimbingKey_C")
  (Input|DisableInput (Game|GetPlayerController 0))
  (Variables|Default|SetRotating false))

(event OnComponentBeginOverlap(Box)
  (params (OverlappedComponent :type Primitive%20Component%20Object%20Reference) (OtherActor :type Actor%20Object%20Reference) (OtherComp :type Primitive%20Component%20Object%20Reference) (OtherBodyIndex :type Integer) (bFromSweep :type Boolean) (SweepResult :type Hit%20Result%20Structure%20%28by%20ref%29))
  ;[0.15 0.15 0.15 0.5] Displaying controls
  (bind _asbp_first_person_character (Utilities|Casting|CastToBP_FirstPersonCharacter OtherActor))
  (Default|VisibleWidget _asbp_first_person_character "/Game/Climbing/ClimbingKey.ClimbingKey_C")
  (Input|EnableInput (Game|GetPlayerController 0))
  (Variables|Default|SetRotating true)
  (CallFunction|RotatingWherePlayerIs))

(event Custom|RotatingWherePlayerIs
  (bind _returnvalue (Transformation|GetActorRotation))
  ;[0.15 0.15 0.15 0.5] Rotating Spline Path
  (if (Variables|Default|GetRotating) :!label _label
    (bind _returnvalue_2 (Actor|GetActorOfClass "/Game/FirstPerson/Blueprints/BP_FirstPersonCharacter.BP_FirstPersonCharacter_C"))
    (Transformation|SetWorldRotation (Variables|Default|GetArrow) (Math|Rotator|MakeRotator (.roll _returnvalue) (.pitch _returnvalue) (.yaw (Math|Rotator|FindLookatRotation (Transformation|GetActorLocation) (Transformation|GetActorLocation _returnvalue_2)))) false false)
    (Utilities|FlowControl|Delay 0.1)
    (goto _label)))

(event Custom|ClimbingEvent
  (bind _climbingpath (Variables|Default|GetClimbingPath))
  ;[0.15 0.15 0.15 0.5] Moving the Player
  (bind _returnvalue (Actor|GetActorOfClass "/Game/FirstPerson/Blueprints/BP_FirstPersonCharacter.BP_FirstPersonCharacter_C"))
  (Variables|Default|SetPlayerReference _returnvalue)
  (Utilities|FlowControl|Sequence
    (:then_0
      (bind _newtrack_0 (Timeline|Climbing PlayFromStart)
        (:Update
          (Transformation|SetActorLocation (Variables|Default|GetPlayerReference) (Math|Vector|MakeVector (.x (Spline|GetLocationatDistanceAlongSpline _climbingpath (Math|Float|Lerp 0.0 (Spline|GetSplineLength _climbingpath) _newtrack_0) "World")) (.y (Spline|GetLocationatDistanceAlongSpline _climbingpath (Math|Float|Lerp 0.0 (Spline|GetSplineLength _climbingpath) _newtrack_0) "World")) (.z (Spline|GetLocationatDistanceAlongSpline _climbingpath (Math|Float|Lerp 0.0 (Spline|GetSplineLength _climbingpath) _newtrack_0) "World"))) false false))))
    (:then_1
      (bind _output_get (Variables|Default|SetCameraRotationYCopyBefore (.pitch (Transformation|GetWorldRotation (Variables|/Game/FirstPerson/Blueprints/BP_FirstPersonCharacter.BP_FirstPersonCharacter_C|GetFirstPersonCamera (Variables|Default|GetPlayerReference))))))
      (Input|DisableInput (Variables|Default|GetPlayerReference) (Game|GetPlayerController 0))
      (Variables|/Script/Engine.Pawn|SetbUseControllerRotationPitch (Variables|Default|GetPlayerReference) true)
      (Variables|/Script/Engine.CameraComponent|SetbUsePawnControlRotation (Variables|/Game/FirstPerson/Blueprints/BP_FirstPersonCharacter.BP_FirstPersonCharacter_C|GetFirstPersonCamera (Variables|Default|GetPlayerReference)) false)
      (bind _newtrack_0_2 (Timeline|CameraRotation PlayFromStart)
        (:Update
          (Transformation|SetWorldRotation (Variables|/Game/FirstPerson/Blueprints/BP_FirstPersonCharacter.BP_FirstPersonCharacter_C|GetFirstPersonCamera (Variables|Default|GetPlayerReference)) (Math|Rotator|MakeRotator (.roll (Transformation|GetWorldRotation (Variables|/Game/FirstPerson/Blueprints/BP_FirstPersonCharacter.BP_FirstPersonCharacter_C|GetFirstPersonCamera (Variables|Default|GetPlayerReference)))) (Math|Float|Lerp _output_get -4e+01 _newtrack_0_2) (.yaw (Transformation|GetWorldRotation (Variables|/Game/FirstPerson/Blueprints/BP_FirstPersonCharacter.BP_FirstPersonCharacter_C|GetFirstPersonCamera (Variables|Default|GetPlayerReference))))) false false)
          (Variables|/Script/Engine.Pawn|SetbUseControllerRotationPitch (Variables|Default|GetPlayerReference) false)
          (Utilities|FlowControl|Delay 1.0)
          (Variables|/Script/Engine.CameraComponent|SetbUsePawnControlRotation (Variables|/Game/FirstPerson/Blueprints/BP_FirstPersonCharacter.BP_FirstPersonCharacter_C|GetFirstPersonCamera (Variables|Default|GetPlayerReference)) true)
          (Input|EnableInput (Variables|Default|GetPlayerReference) (Game|GetPlayerController 0)))))))

(fn ConstructionScript)