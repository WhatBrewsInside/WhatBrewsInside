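; Switchable spotlight actor that can be turned on and off through its ToggleLights event.
; ToggleLights flips the IsOn flag, applies it to the SpotLight's visibility and sets the light's color from LightColor.
; The construction script applies IsOn to visibility so the initial state matches the flag, but leaves the color untouched until a toggle.
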(event EventToggleLights
  (bind _output_get (Variables|Default|SetIsOn (not (Variables|Default|GetIsOn))))
  (Rendering|SetVisibility (Variables|Default|GetSpotLight) _output_get false)
  (Rendering|Components|Light|SetLightColor (Variables|Default|GetSpotLight) (Variables|Default|GetLightColor) true))

(fn ConstructionScript
  (Rendering|SetVisibility (Variables|Default|GetSpotLight) (Variables|Default|GetIsOn) false))