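; Light switch actor that lets the first-person player toggle linked lights by pressing E while inside its box trigger.
; BeginPlay caches every Light_BP in the level into an array.
; Box overlap shows or hides the SwitchKey prompt, enables or disables input, and opens or closes a Gate for the E key.
; A press through the open Gate calls ToggleLightsMessage on every cached light whose LightIndex matches the switch's.
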(event OnComponentBeginOverlap(Box)
  (params (OverlappedComponent :type Primitive%20Component%20Object%20Reference) (OtherActor :type Actor%20Object%20Reference) (OtherComp :type Primitive%20Component%20Object%20Reference) (OtherBodyIndex :type Integer) (bFromSweep :type Boolean) (SweepResult :type Hit%20Result%20Structure%20%28by%20ref%29))
  ;[0.15 0.15 0.15 0.5] Displaying controls
  (bind _asbp_first_person_character (Utilities|Casting|CastToBP_FirstPersonCharacter OtherActor))
  (Default|VisibleWidget _asbp_first_person_character "/Game/Switches/SwitchKey.SwitchKey_C")
  (Input|EnableInput (Game|GetPlayerController 0))
  ;[0.15 0.15 0.15 0.5] Checking if the switch and the light have the same index and then turning on the correct lights
  (Utilities|FlowControl|Gate true) ; enters at Open
)

(event OnComponentEndOverlap(Box)
  (params (OverlappedComponent :type Primitive%20Component%20Object%20Reference) (OtherActor :type Actor%20Object%20Reference) (OtherComp :type Primitive%20Component%20Object%20Reference) (OtherBodyIndex :type Integer))
  ;[0.15 0.15 0.15 0.5] Displaying controls
  (bind _asbp_first_person_character (Utilities|Casting|CastToBP_FirstPersonCharacter OtherActor))
  (Default|HiddenWidget _asbp_first_person_character "/Game/Switches/SwitchKey.SwitchKey_C")
  (Input|DisableInput (Game|GetPlayerController 0))
  ;[0.15 0.15 0.15 0.5] Checking if the switch and the light have the same index and then turning on the correct lights
  (Utilities|FlowControl|Gate true) ; enters at Close
)

(event EventBeginPlay
  ;[0.15 0.15 0.15 0.5] Adding lights to an array of lights
  (bind _outactors (Actor|GetAllActorsOfClass "/Game/Switches/Light_BP.Light_BP_C"))
  (for _array_element _outactors
    (Utilities|Array|Add (Variables|Default|GetLightArray) _array_element)))

(event Input|KeyboardEvents|E
  (params (Key :type Key%20Structure :default "None"))
  ;[0.15 0.15 0.15 0.5] Checking if the switch and the light have the same index and then turning on the correct lights
  (:Pressed
    (Utilities|FlowControl|Gate true
      (:Exit
        (for _array_element (Variables|Default|GetLightArray)
          (if (== (Variables|/Game/Switches/Light_BP.Light_BP_C|GetLightIndex _array_element) (Variables|Default|GetLightIndex))
            (Class|LightsInterface|ToggleLights(Message) _array_element)))))))

(fn ConstructionScript)