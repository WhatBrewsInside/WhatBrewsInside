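; BP_EnemyPrototype is a prototype enemy that damages the first-person player on touch and turns toward them.
; Capsule overlap clears the highest active of three HealthBarArray slots, updates WB_HealthBar, then blocks further hits briefly via WasHit.
; Entering NoticingArea plays one of two timelines, chosen by look-at yaw, to lerp rotation toward the player with a quarter-turn offset.
; The delayed repeat of this rotation is disconnected, so it triggers only on entry.
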(event OnComponentBeginOverlap(Capsule)
  (params (OverlappedComponent :type Primitive%20Component%20Object%20Reference) (OtherActor :type Actor%20Object%20Reference) (OtherComp :type Primitive%20Component%20Object%20Reference) (OtherBodyIndex :type Integer) (bFromSweep :type Boolean) (SweepResult :type Hit%20Result%20Structure%20%28by%20ref%29))
  (bind _asbp_first_person_character (Utilities|Casting|CastToBP_FirstPersonCharacter OtherActor))
  (if (not (Variables|Default|GetWasHit?))
    (if (== (Utilities|Array|Get(acopy) (Variables|/Game/FirstPerson/Blueprints/BP_FirstPersonCharacter.BP_FirstPersonCharacter_C|GetHealthBarArray _asbp_first_person_character) 2) true)
      (bind _foundwidgets (Widget|GetAllWidgetsOfClass "/Game/Widgets/WB_HealthBar.WB_HealthBar_C" true))
      (Default|TurningOfHealth _foundwidgets 2)
      (bind _returnvalue (Actor|GetActorOfClass "/Game/FirstPerson/Blueprints/BP_FirstPersonCharacter.BP_FirstPersonCharacter_C"))
      (Utilities|Array|SetArrayElem (Variables|/Game/FirstPerson/Blueprints/BP_FirstPersonCharacter.BP_FirstPersonCharacter_C|GetHealthBarArray _returnvalue) 2 false)
      (Variables|Default|SetWasHit? true :!label _label)
      (Utilities|FlowControl|Delay 1.0)
      (Variables|Default|SetWasHit? false)
      (elif (== (Utilities|Array|Get(acopy) (Variables|/Game/FirstPerson/Blueprints/BP_FirstPersonCharacter.BP_FirstPersonCharacter_C|GetHealthBarArray _asbp_first_person_character) 1) true)
        (bind _foundwidgets_2 (Widget|GetAllWidgetsOfClass "/Game/Widgets/WB_HealthBar.WB_HealthBar_C" true))
        (Default|TurningOfHealth _foundwidgets_2 1)
        (bind _returnvalue_2 (Actor|GetActorOfClass "/Game/FirstPerson/Blueprints/BP_FirstPersonCharacter.BP_FirstPersonCharacter_C"))
        (Utilities|Array|SetArrayElem (Variables|/Game/FirstPerson/Blueprints/BP_FirstPersonCharacter.BP_FirstPersonCharacter_C|GetHealthBarArray _returnvalue_2) 1 false)
        (goto _label)
        (elif (== (Utilities|Array|Get(acopy) (Variables|/Game/FirstPerson/Blueprints/BP_FirstPersonCharacter.BP_FirstPersonCharacter_C|GetHealthBarArray _asbp_first_person_character)) true)
          (bind _foundwidgets_3 (Widget|GetAllWidgetsOfClass "/Game/Widgets/WB_HealthBar.WB_HealthBar_C" true))
          (Default|TurningOfHealth _foundwidgets_3)
          (bind _returnvalue_3 (Actor|GetActorOfClass "/Game/FirstPerson/Blueprints/BP_FirstPersonCharacter.BP_FirstPersonCharacter_C"))
          (Utilities|Array|SetArrayElem (Variables|/Game/FirstPerson/Blueprints/BP_FirstPersonCharacter.BP_FirstPersonCharacter_C|GetHealthBarArray _returnvalue_3) 0 false)
          (goto _label))))))

(event OnComponentEndOverlap(NoticingArea)
  (params (OverlappedComponent :type Primitive%20Component%20Object%20Reference) (OtherActor :type Actor%20Object%20Reference) (OtherComp :type Primitive%20Component%20Object%20Reference) (OtherBodyIndex :type Integer))
  (Variables|Default|SetIsInZone? false))

(event OnComponentBeginOverlap(NoticingArea)
  (params (OverlappedComponent :type Primitive%20Component%20Object%20Reference) (OtherActor :type Actor%20Object%20Reference) (OtherComp :type Primitive%20Component%20Object%20Reference) (OtherBodyIndex :type Integer) (bFromSweep :type Boolean) (SweepResult :type Hit%20Result%20Structure%20%28by%20ref%29))
  (bind _asbp_first_person_character (Utilities|Casting|CastToBP_FirstPersonCharacter OtherActor))
  (Variables|Default|SetOther%20Actor _asbp_first_person_character)
  (Variables|Default|SetIsInZone? true)
  (CallFunction|RepeatActionLoop))

(event Custom|RepeatActionLoop
  (bind _returnvalue (Transformation|GetActorLocation))
  (bind _returnvalue_2 (Transformation|GetActorRotation))
  (bind _other_actor (Variables|Default|GetOther%20Actor))
  (bind _returnvalue_3 (Transformation|GetActorLocation _other_actor))
  (bind _returnvalue_4 (Math|Rotator|FindLookatRotation _returnvalue _returnvalue_3))
  ;[0.15 0.15 0.15 0.5] Rotating enemy towards player
  (if (Variables|Default|GetIsInZone?)
    (if (< (.yaw _returnvalue_4) -9e+01)
      (bind _newtrack_0 (Timeline|Rotating PlayFromStart)
        (:Update
          (Transformation|SetActorRotation (Math|Rotator|MakeRotator 0.0 0.0 (.yaw (Math|Rotator|Lerp(Rotator) (Math|Rotator|MakeRotator 0.0 0.0 (.yaw _returnvalue_2)) (Math|Rotator|MakeRotator 0.0 0.0 (+ (.yaw _returnvalue_4) 2.7e+02)) _newtrack_0 true))))))
      (else
        (bind _newtrack_0_2 (Timeline|Timeline PlayFromStart)
          (:Update
            (Transformation|SetActorRotation (Math|Rotator|MakeRotator 0.0 0.0 (.yaw (Math|Rotator|Lerp(Rotator) (Math|Rotator|MakeRotator 0.0 0.0 (.yaw _returnvalue_2)) (Math|Rotator|MakeRotator 0.0 0.0 (- (.yaw _returnvalue_4) 9e+01)) _newtrack_0_2 true))))))))))

(event Collision|EventActorBeginOverlap
  (params (OtherActor :type Actor%20Object%20Reference)))

(fn ConstructionScript)