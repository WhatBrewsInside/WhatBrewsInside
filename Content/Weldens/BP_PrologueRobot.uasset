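; Prologue robot character that stages a one-time reveal cutscene when the player enters its sphere, then chases them.
; The overlap disables input and blends the view to a spawned camera at the player's viewpoint, aimed at the robot.
; After blending back and restoring input, it destroys that camera and repeatedly issues AIMoveTo toward the player.
; The kill and head-turn animation is only a print placeholder, and an older timeline-based player rotation is disconnected.
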(event OnComponentBeginOverlap(Sphere)
  (params (OverlappedComponent :type Primitive%20Component%20Object%20Reference) (OtherActor :type Actor%20Object%20Reference) (OtherComp :type Primitive%20Component%20Object%20Reference) (OtherBodyIndex :type Integer) (bFromSweep :type Boolean) (SweepResult :type Hit%20Result%20Structure%20%28by%20ref%29))
  (bind _asbp_first_person_character (Utilities|Casting|CastToBP_FirstPersonCharacter OtherActor))
  (if (Variables|Default|GetFirstTime?)
    (bind _output_get (Variables|Default|SetPlayer _asbp_first_person_character))
    (Development|PrintString (Utilities|String|ToString(Vector) (Variables|/Script/Engine.SceneComponent|GetRelativeLocation (Variables|/Game/FirstPerson/Blueprints/BP_FirstPersonCharacter.BP_FirstPersonCharacter_C|GetFirstPersonCamera _output_get))))
    (Input|DisableInput (Variables|Default|GetPlayer) (Game|GetPlayerController 0))
    (Variables|Default|SetFirstTime? false)
    (bind _returnvalue (Game|SpawnActorfromClass "/Script/Engine.CameraActor" (Math|Transform|MakeTransform (.location (Transformation|GetWorldTransform (Variables|/Game/FirstPerson/Blueprints/BP_FirstPersonCharacter.BP_FirstPersonCharacter_C|GetFirstPersonCamera _asbp_first_person_character))) (Math|Rotator|FindLookatRotation (.location (Transformation|GetWorldTransform (Variables|/Game/FirstPerson/Blueprints/BP_FirstPersonCharacter.BP_FirstPersonCharacter_C|GetFirstPersonCamera _asbp_first_person_character))) (Transformation|GetActorLocation)) (.scale (Transformation|GetWorldTransform (Variables|/Game/FirstPerson/Blueprints/BP_FirstPersonCharacter.BP_FirstPersonCharacter_C|GetFirstPersonCamera _asbp_first_person_character)))) "Undefined" "MultiplyWithRoot" 0 (Variables|Default|GetPlayer)))
    (Utilities|FlowControl|Sequence
      (:then_0
        (Transformation|AttachComponentToComponent (Variables|/Script/Engine.CameraActor|GetCameraComponent _returnvalue) (Variables|/Script/Engine.Character|GetMesh (Variables|Default|GetPlayer)) "" "KeepWorld" "KeepWorld" "KeepWorld" false)
        (Game|Player|SetViewTargetwithBlend (Game|GetPlayerController 0) _returnvalue 1.0 "VTBlend_Cubic" 0.0 true)
        (Utilities|FlowControl|Delay 2.5)
        (Game|Player|SetViewTargetwithBlend (Game|GetPlayerController 0) (Variables|Default|GetPlayer) 0.2 "VTBlend_Cubic" 0.0 false)
        (Utilities|FlowControl|Delay 0.2)
        (Input|EnableInput (Variables|Default|GetPlayer) (Game|GetPlayerController 0))
        (Actor|DestroyActor _returnvalue)
        (CallFunction|Chasing))
      (:then_1
        (Utilities|FlowControl|Delay 1.0)
        (Utilities|FlowControl|Delay 2.5)
        (Development|PrintString "Animacja mordowania i odwrócenia głowy")
        (Utilities|FlowControl|Delay 0.4)))))

(event Custom|Chasing
  (bind _returnvalue (Actor|GetActorOfClass "/Game/FirstPerson/Blueprints/BP_FirstPersonCharacter.BP_FirstPersonCharacter_C"))
  (AI|AIMoveTo self (Transformation|GetActorLocation _returnvalue) 0 1.0 false :!label _label
    (:then
      (Utilities|FlowControl|Delay 0.1)
      (goto _label))))

(event EventBeginPlay)

(event Collision|EventActorBeginOverlap
  (params (OtherActor :type Actor%20Object%20Reference)))

(event EventTick
  (params (DeltaSeconds :type Float%20%28single-precision%29)))

(fn ConstructionScript)