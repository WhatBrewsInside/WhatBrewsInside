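; BP_EnemyPrototype2 is a prototype enemy that wanders, investigates noises and chases the player.
; It wanders at slow speed between random points in a hard-coded rectangle.
; PawnSensing sight starts a move to the player; hearing speeds it to the noise, then it resumes wandering.
; Overlapping the FollowingPlayer zone starts a fast chase that repeatedly re-targets the player, while the HearingDistance sphere only visualizes hearing range.
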(event OnHearNoise(PawnSensing)
  (params (Instigator :type Pawn%20Object%20Reference) (Location :type Vector%20%28by%20ref%29 :default "0, 0, 0") (Volume :type Float%20%28single-precision%29))
  ;[0.15 0.15 0.15 0.5] going to where the sound was
  (Variables|/Script/Engine.CharacterMovementComponent|SetMaxWalkSpeed (Variables|Character|GetCharacterMovement) 7e+02)
  (if (not (Variables|Default|GetIsPlayerInFollowingZone?))
    (AI|AIMoveTo self Location 0 5.0 false
      (:OnSuccess
        (Utilities|FlowControl|Delay 2.0)
        (CallFunction|WalkingAround)))))

(event OnSeePawn(PawnSensing)
  (params (Pawn :type Pawn%20Object%20Reference))
  ;[0.15 0.15 0.15 0.5] Moving to player that it has seen
  (Variables|Default|SetIsPlayerInHearingZone? true)
  (CallFunction|FollowPlayer))

(event OnComponentBeginOverlap(FollowingPlayer)
  (params (OverlappedComponent :type Primitive%20Component%20Object%20Reference) (OtherActor :type Actor%20Object%20Reference) (OtherComp :type Primitive%20Component%20Object%20Reference) (OtherBodyIndex :type Integer) (bFromSweep :type Boolean) (SweepResult :type Hit%20Result%20Structure%20%28by%20ref%29))
  ;[0.15 0.15 0.15 0.5] Following player when he is closed to it
  (Utilities|Casting|CastToBP_FirstPersonCharacter OtherActor)
  (Variables|Default|SetIsPlayerInFollowingZone? true)
  (Variables|/Script/Engine.CharacterMovementComponent|SetMaxWalkSpeed (Variables|Character|GetCharacterMovement) 7e+02)
  (if (Variables|Default|GetIsPlayerInFollowingZone?) :!label _label
    (bind _returnvalue (Actor|GetActorOfClass "/Game/FirstPerson/Blueprints/BP_FirstPersonCharacter.BP_FirstPersonCharacter_C"))
    (AI|AIMoveTo self (Transformation|GetActorLocation _returnvalue) 0 0.0 false
      (:then
        (Utilities|FlowControl|Delay 0.1)
        (goto _label)))
    (else
      (CallFunction|WalkingAround))))

(event OnComponentEndOverlap(FollowingPlayer)
  (params (OverlappedComponent :type Primitive%20Component%20Object%20Reference) (OtherActor :type Actor%20Object%20Reference) (OtherComp :type Primitive%20Component%20Object%20Reference) (OtherBodyIndex :type Integer))
  ;[0.15 0.15 0.15 0.5] Following player when he is closed to it
  (Utilities|Casting|CastToBP_FirstPersonCharacter OtherActor)
  (Variables|Default|SetIsPlayerInFollowingZone? false)
  (Variables|/Script/Engine.CharacterMovementComponent|SetMaxWalkSpeed (Variables|Character|GetCharacterMovement) 7e+02))

(event Custom|FollowPlayer
  ;[0.15 0.15 0.15 0.5] Moving to player that it has seen
  (if (Variables|Default|GetIsPlayerInHearingZone?)
    (AI|AIMoveTo self "0, 0, 0" (Game|GetPlayerCharacter 0) 5.0 false)))

(event Custom|WalkingAround
  ;[0.15 0.15 0.15 0.5] walking around
  (Variables|/Script/Engine.CharacterMovementComponent|SetMaxWalkSpeed (Variables|Character|GetCharacterMovement) 3e+02)
  (AI|AIMoveTo self (Math|Vector|MakeVector (Math|Random|RandomFloatinRange 155.0 2844.0) (Math|Random|RandomFloatinRange 5643.0 11948.0) (.z (Transformation|GetActorLocation))) 0 5.0 false :!label _label
    (:OnSuccess
      (Utilities|FlowControl|Delay 0.2)
      (goto _label))))

(event Collision|EventActorBeginOverlap
  (params (OtherActor :type Actor%20Object%20Reference)))

(event EventBeginPlay
  (Utilities|FlowControl|Sequence
    (:then_0
      ;[0.15 0.15 0.15 0.5] setting HearingDistance(collison sphere, I added this to visualy represent distance of hearing, it has no other functions than that) to hearing threshold(distance) of enemy
      (Components|Sphere|SetSphereRadius (Variables|Default|GetHearingDistance) (Variables|/Script/AIModule.PawnSensingComponent|GetHearingThreshold (Variables|Default|GetPawnSensing)) true))
    (:then_1
      (CallFunction|WalkingAround))))

(fn ConstructionScript)