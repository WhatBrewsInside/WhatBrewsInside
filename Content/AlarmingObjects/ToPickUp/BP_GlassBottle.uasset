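; Glass bottle pickup that shows itself in the inventory bar when the first-person character overlaps it, then destroys itself.
; The overlap fills the WB_InventoryBar name and quantity texts, reading HowManyBottles from the character without changing it.
; A switch on InventoryBarIndex sets a placeholder Android icon on one of five slot images.
; Each branch wires a short Delay back into the widget update after DestroyActor.
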(event OnComponentBeginOverlap(GlassBottle)
  (params (OverlappedComponent :type Primitive%20Component%20Object%20Reference) (OtherActor :type Actor%20Object%20Reference) (OtherComp :type Primitive%20Component%20Object%20Reference) (OtherBodyIndex :type Integer) (bFromSweep :type Boolean) (SweepResult :type Hit%20Result%20Structure%20%28by%20ref%29))
  (bind _asbp_first_person_character (Utilities|Casting|CastToBP_FirstPersonCharacter OtherActor))
  (bind _foundwidgets (Widget|GetAllWidgetsOfClass "/Game/Widgets/WB_InventoryBar.WB_InventoryBar_C" true :!label _label))
  (Variables|Default|SetNameOfItem (Utilities|Text|ToText(Object) OverlappedComponent))
  (Class|TextBlock|SetOpacity (Variables|/Game/Widgets/WB_InventoryBar.WB_InventoryBar_C|GetNameOfItem (Utilities|Array|Get(acopy) _foundwidgets)) 1e+02)
  (Rendering|Components|TextRender|SetText (Variables|/Game/Widgets/WB_InventoryBar.WB_InventoryBar_C|GetNameOfItem (Utilities|Array|Get(acopy) _foundwidgets)) (Variables|Default|GetNameOfItem))
  (Class|TextBlock|SetOpacity (Variables|/Game/Widgets/WB_InventoryBar.WB_InventoryBar_C|GetQuantityOfItem (Utilities|Array|Get(acopy) _foundwidgets)) 1e+02)
  (bind _returnvalue (Actor|GetActorOfClass "/Game/FirstPerson/Blueprints/BP_FirstPersonCharacter.BP_FirstPersonCharacter_C"))
  (Rendering|Components|TextRender|SetText (Variables|/Game/Widgets/WB_InventoryBar.WB_InventoryBar_C|GetQuantityOfItem (Utilities|Array|Get(acopy) _foundwidgets)) (Utilities|Text|ToText(Integer) (Variables|/Game/FirstPerson/Blueprints/BP_FirstPersonCharacter.BP_FirstPersonCharacter_C|GetHowManyBottles _returnvalue)))
  (switch int (Variables|/Game/Widgets/WB_InventoryBar.WB_InventoryBar_C|GetInventoryBarIndex (Utilities|Array|Get(acopy) _foundwidgets))
    (:0
      (Class|Image|SetOpacity (Variables|/Game/Widgets/WB_InventoryBar.WB_InventoryBar_C|GetImage1 (Utilities|Array|Get(acopy) _foundwidgets)) 1e+02)
      (Appearance|SetBrushfromTexture (Variables|/Game/Widgets/WB_InventoryBar.WB_InventoryBar_C|GetImage1 (Utilities|Array|Get(acopy) _foundwidgets)) "/Engine/Tutorial/Mobile/TutorialAssets/android_Icon.android_Icon" true)
      (Actor|DestroyActor)
      (Utilities|FlowControl|Delay 0.1)
      (goto _label))
    (:1
      (Class|Image|SetOpacity (Variables|/Game/Widgets/WB_InventoryBar.WB_InventoryBar_C|GetImage2 (Utilities|Array|Get(acopy) _foundwidgets)) 1e+02)
      (Appearance|SetBrushfromTexture (Variables|/Game/Widgets/WB_InventoryBar.WB_InventoryBar_C|GetImage2 (Utilities|Array|Get(acopy) _foundwidgets)) "/Engine/Tutorial/Mobile/TutorialAssets/android_Icon.android_Icon" true)
      (Actor|DestroyActor)
      (Utilities|FlowControl|Delay 0.1)
      (goto _label))
    (:2
      (Class|Image|SetOpacity (Variables|/Game/Widgets/WB_InventoryBar.WB_InventoryBar_C|GetImage3 (Utilities|Array|Get(acopy) _foundwidgets)) 1e+02)
      (Appearance|SetBrushfromTexture (Variables|/Game/Widgets/WB_InventoryBar.WB_InventoryBar_C|GetImage3 (Utilities|Array|Get(acopy) _foundwidgets)) "/Engine/Tutorial/Mobile/TutorialAssets/android_Icon.android_Icon" true)
      (Actor|DestroyActor)
      (Utilities|FlowControl|Delay 0.1)
      (goto _label))
    (:3
      (Class|Image|SetOpacity (Variables|/Game/Widgets/WB_InventoryBar.WB_InventoryBar_C|GetImage4 (Utilities|Array|Get(acopy) _foundwidgets)) 1e+02)
      (Appearance|SetBrushfromTexture (Variables|/Game/Widgets/WB_InventoryBar.WB_InventoryBar_C|GetImage4 (Utilities|Array|Get(acopy) _foundwidgets)) "/Engine/Tutorial/Mobile/TutorialAssets/android_Icon.android_Icon" true)
      (Actor|DestroyActor)
      (Utilities|FlowControl|Delay 0.1)
      (goto _label))
    (:4
      (Class|Image|SetOpacity (Variables|/Game/Widgets/WB_InventoryBar.WB_InventoryBar_C|GetImage5 (Utilities|Array|Get(acopy) _foundwidgets)) 1e+02)
      (Appearance|SetBrushfromTexture (Variables|/Game/Widgets/WB_InventoryBar.WB_InventoryBar_C|GetImage5 (Utilities|Array|Get(acopy) _foundwidgets)) "/Engine/Tutorial/Mobile/TutorialAssets/android_Icon.android_Icon" true)
      (Actor|DestroyActor)
      (Utilities|FlowControl|Delay 0.1)
      (goto _label))))

(event EventBeginPlay)

(event Collision|EventActorBeginOverlap
  (params (OtherActor :type Actor%20Object%20Reference)))

(event EventTick
  (params (DeltaSeconds :type Float%20%28single-precision%29)))

(fn ConstructionScript)