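; Parent Blueprint for throwable objects that shatter or break on impact and make noise that can alert AI.
; When the static mesh hits something, the object destroys itself, spawns its configured replacement class at that location and plays its sound quietly with shattered-glass attenuation.
; It then reports a noise at the impact point through the first-person character's PawnNoiseEmitter, found with GetActorOfClass, naming itself as noise maker.
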(event OnComponentHit(StaticMesh)
  (params (HitComponent :type Primitive%20Component%20Object%20Reference) (OtherActor :type Actor%20Object%20Reference) (OtherComp :type Primitive%20Component%20Object%20Reference) (NormalImpulse :type Vector :default "0, 0, 0") (Hit :type Hit%20Result%20Structure%20%28by%20ref%29))
  (Variables|Default|SetObjet'sTransform (Transformation|GetWorldTransform (Variables|Default|GetStaticMesh)))
  (Actor|DestroyActor)
  (Game|SpawnActorfromClass (Variables|Default|GetSpawnedAfterHit) (Math|Transform|MakeTransform (.location (Variables|Default|GetObjet'sTransform)) "0, 0, 0" "1.000000,1.000000,1.000000") "Undefined" "MultiplyWithRoot" 0 0)
  (bind _returnvalue (Actor|GetActorOfClass "/Game/FirstPerson/Blueprints/BP_FirstPersonCharacter.BP_FirstPersonCharacter_C"))
  (Audio|PlaySoundatLocation (Variables|Default|GetSound) (.location (Variables|Default|GetObjet'sTransform)) "0, 0, 0" 0.1 1.0 0.0 "/Game/AlarmingObjects/SA_ShatteredGlass.SA_ShatteredGlass" 0 0 0)
  (Class|PawnNoiseEmitterComponent|MakeNoise (Variables|/Game/FirstPerson/Blueprints/BP_FirstPersonCharacter.BP_FirstPersonCharacter_C|GetPawnNoiseEmitter _returnvalue) self 1.0 (.location (Variables|Default|GetObjet'sTransform))))

(event Collision|EventActorBeginOverlap
  (params (OtherActor :type Actor%20Object%20Reference)))

(fn ConstructionScript)