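; Inventory component that stores item stacks in a map keyed by data asset Index and toggles the inventory screen.
; BeginPlay adds the inventory input mapping; its action creates or removes UMG_Inventory, switching cursor and input mode.
; PickUpItem adds missing keys, checks capacity through IsKeyFull against MaxStack, and returns whether the item was consumed plus any leftover.
; Its stack write sums the incoming quantity with itself, ignoring the stored amount.
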(event Input|EnhancedActionEvents|EnhancedInputActionIA_Inventory
  (params (ActionValue :type Boolean) (ElapsedSeconds :type Float%20%28double-precision%29) (TriggeredSeconds :type Float%20%28double-precision%29) (InputAction :type Input%20Action%20Object%20Reference :default "/Game/Inventory/IA_Inventory.IA_Inventory"))
  (bind _returnvalue (Game|GetPlayerController 0))
  (bind _returnvalue_2 (Game|GetPlayerController 0))
  (:Started
    (Variables|Default|Getas%20UMG_Inventory
      (:then
        (Variables|/Script/Engine.PlayerController|SetbShowMouseCursor _returnvalue_2 false)
        (Input|SetInputModeGameOnly _returnvalue_2 false)
        (Widget|RemovefromParent (Variables|Default|Getas%20UMG_Inventory))
        (Variables|Default|Setas%20UMG_Inventory 0))
      (:else
        (bind _returnvalue_3 (UserInterface|CreateWidget "/Game/Inventory/Widgets/UMG_Inventory.UMG_Inventory_C"))
        (bind _output_get (Variables|Default|Setas%20UMG_Inventory _returnvalue_3))
        (UserInterface|Viewport|AddtoViewport _output_get 0)
        (Variables|/Script/Engine.PlayerController|SetbShowMouseCursor _returnvalue true)
        (Input|SetInputModeGameandUI _returnvalue 0 "DoNotLock" true false)))))

(event EventBeginPlay
  ;[0.15 0.15 0.15 0.5] Add key bindings
  (Input|AddMappingContext (PlayerController|LocalPlayerSubsystems|GetEnhancedInputLocalPlayerSubsystem (Game|GetPlayerController 0)) "/Game/Inventory/IMC_Inventory.IMC_Inventory" 0 "(bIgnoreAllPressedKeysUntilRelease=True,bForceImmediately=False,bNotifyUserSettings=False)"))

(fn PickUpItem
  (params (Item :type A%20Item%20Object%20Reference))
  (bind _structure (Variables|/Game/Inventory/Items/A_Item.A_Item_C|GetStructure Item))
  (bind (_quantity _dataasset) (Utilities|Struct|BreakST_Item _structure))
  (bind _structure_2 (Variables|/Game/Inventory/Items/A_Item.A_Item_C|GetStructure Item))
  (bind _structure_3 (Variables|/Game/Inventory/Items/A_Item.A_Item_C|GetStructure Item))
  (bind (_quantity_2 _dataasset_2 _index) (Utilities|Struct|BreakST_Item _structure_2))
  (bind (_quantity_3 _dataasset_3 _index_2) (Utilities|Struct|BreakST_Item _structure_3))
  ;[0.15 0.15 0.15 0.5] Wild shit
  (LocalVariables|SetL-QuantityIn _quantity)
  (LocalVariables|SetL-dataAsset _dataasset)
  (bind _output_get (LocalVariables|SetL-Index (Variables|/Game/Inventory/Items/DA_Items.DA_Items_C|GetIndex _dataasset)))
  (if (.ReturnValue (Utilities|Map|Find (Variables|Default|GetInventory) _output_get))
    _
    (else
      (CallFunction|ItemAdded (LocalVariables|GetL-Index) _structure)))
  (bind (_returnvalue _remainingquantity) (CallFunction|IsKeyFull (LocalVariables|GetL-Index)))
  (LocalVariables|SetL-RemainingQuantity _remainingquantity)
  (if _returnvalue
    (return false (LocalVariables|GetL-QuantityIn))
    (elif (<= (LocalVariables|GetL-QuantityIn) _remainingquantity)
      (Utilities|Map|Add (Variables|Default|GetInventory) (LocalVariables|GetL-Index) (Utilities|Struct|MakeST_Item (+ (LocalVariables|GetL-QuantityIn) _quantity_3) _dataasset_3 _index_2))
      (return true 0)
      (else
        (Utilities|Map|Add (Variables|Default|GetInventory) (LocalVariables|GetL-Index) (Utilities|Struct|MakeST_Item (Variables|/Game/Inventory/Items/DA_Items.DA_Items_C|GetMaxStack (.DataAsset (Utilities|Struct|BreakST_Item _structure_2))) _dataasset_2 _index))
        (return true (- (LocalVariables|GetL-QuantityIn) (LocalVariables|GetL-RemainingQuantity)))))))

(fn IsKeyFull
  (params (Key :type Integer))
  (bind _inventory (Variables|Default|GetInventory))
  (bind (_value _returnvalue) (Utilities|Map|Find _inventory Key))
  (bind (_quantity _dataasset) (Utilities|Struct|BreakST_Item _value))
  (bind _maxstack (Variables|/Game/Inventory/Items/DA_Items.DA_Items_C|GetMaxStack _dataasset))
  (bind _returnvalue_2 (- _maxstack _quantity))
  (if _returnvalue
    (return (and (== _returnvalue_2 0) (!= _maxstack 0)) _returnvalue_2)
    (else
      (return false -1))))

(fn ItemAdded
  (params (SlotKey :type Integer) (SlotValue :type ST%20Item%20Structure))
  (Utilities|Map|Add (Variables|Default|GetInventory) SlotKey SlotValue))

(fn ItemRemoved
  (params (Key :type Integer))
  (Utilities|Map|Remove (Variables|Default|GetInventory) Key))